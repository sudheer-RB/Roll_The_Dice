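; BP_TileGenerator builds a board grid of tiles and highlights the tiles within reach of the player's rolled number.
; The construction script lays out preview cubes by row and column count, which BeginPlay replaces with BP_Tile actors carrying grid positions.
; HighlightTiles reads the player pawn's current tile, clears old highlights, then highlights other tiles in the same row or column within the roll distance.
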(event `self.ReceiveBeginPlay`
  (for _array_element (`self.tile_cube_preview_meshes`)
    (bind (_relativelocation_x _relativelocation_y) (`KismetMathLibrary.BreakVector` (`SceneComponent.RelativeLocation` _array_element)))
    (bind _returnvalue (`|SpawnActorFromClass` "/Game/Blueprints/BP_Tile.BP_Tile_C" (`SceneComponent.K2_GetComponentToWorld` _array_element) "AlwaysSpawn" "MultiplyWithRoot" self (`StaticMeshComponent.StaticMesh` _array_element) (`KismetMathLibrary.MakeVector2D` (/ _relativelocation_x 100.0) (/ _relativelocation_y 100.0)) false (`self.GetInstigator`)))
    (`KismetArrayLibrary.Array_Add` (`self.tiles`) _returnvalue)
    (`ActorComponent.K2_DestroyComponent` _array_element)))

(fn `Check_Is_Tile_In_Range`
  (params (current :type Integer) (min :type Integer) (max :type Integer))
  (returns (bool :type Boolean))
  (return (and (< current max) (> current min))))

(fn `Highlight_Tiles`
  (params (rolled_num :type Integer))
  (locals (player_tile_pos :type "Vector2D Structure") (current_tile_pos :type "Vector2D Structure"))
  (bind _player_tile_pos (`local.player_tile_pos`))
  (bind (_x _y) (`KismetMathLibrary.BreakVector2D` (`local.player_tile_pos`)))
  (bind (_x_2 _y_2) (`KismetMathLibrary.BreakVector2D` _player_tile_pos))
  (bind (_x_3 _y_3) (`KismetMathLibrary.BreakVector2D` (`local.current_tile_pos`)))
  (bind _returnvalue (+ (`local.rolled_num`) 1))
  (bind _tile_pos (message `/Game/Blueprints/BPI_MyInterface.Get_Player_Current_Tile` (`GameplayStatics.GetPlayerPawn` 0)))
  (set `local.player_tile_pos` _tile_pos)
  (for _array_element (`self.tiles`)
    (`/Game/Blueprints/BP_Tile.UnHighlight_Tile` _array_element))
  (for _array_element_2 (`self.tiles`)
    (bind _tile_pos_2 (`/Game/Blueprints/BP_Tile.tile_pos` _array_element_2))
    (if (not (`self.Is_Pos_Same` _tile_pos_2 _player_tile_pos))
      (bind (_x_4 _y_4) (`KismetMathLibrary.BreakVector2D` _tile_pos_2))
      (if (and (`self.Check_Is_Tile_In_Range` (`KismetMathLibrary.FTrunc` _x_4) (`KismetMathLibrary.FTrunc` (- _x_2 _returnvalue)) (`KismetMathLibrary.FTrunc` (+ _x_2 _returnvalue))) (`self.Check_Is_Tile_In_Range` (`KismetMathLibrary.FTrunc` _y_4) (`KismetMathLibrary.FTrunc` (- _y_2 _returnvalue)) (`KismetMathLibrary.FTrunc` (+ _y_2 _returnvalue))))
        (set `local.current_tile_pos` _tile_pos_2)
        (if (or (== _x_3 _x) (== _y_3 _y))
          (`/Game/Blueprints/BP_Tile.Highlight_Tile` _array_element_2))))))

(fn `Is_Pos_Same`
  (params (a :type "Vector2D Structure") (b :type "Vector2D Structure"))
  (returns (bool :type Boolean))
  (return (and (== a_X b_X) (== a_Y b_Y))))

(fn `Total_Tiles`
  (returns (ReturnValue :type Integer))
  (return (+ (`self.no_of_rows`) (`self.no_of_cols`))))

(fn `UserConstructionScript`
  (`KismetArrayLibrary.Array_Clear` (`self.tile_cube_preview_meshes`))
  (for _index (range 1 (+ (`self.no_of_cols`) 1))
    (for _index_2 (range 1 (+ (`self.no_of_rows`) 1))
      (bind _returnvalue (`AddComponent|NODE_AddStaticMeshComponent-0` :`RelativeTransform` (`KismetMathLibrary.MakeTransform` (`KismetMathLibrary.MakeVector` (`KismetMathLibrary.Conv_IntToDouble` (* _index_2 100)) (`KismetMathLibrary.Conv_IntToDouble` (* _index 100))) (struct) (0.8 0.8 0.3))))
      (`StaticMeshComponent.SetStaticMesh` _returnvalue "/Engine/BasicShapes/Cube.Cube")
      (`KismetArrayLibrary.Array_AddUnique` (`self.tile_cube_preview_meshes`) _returnvalue))))