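; Grid tile actor for click-to-move: clicking a highlighted tile sends its location and grid position to the player pawn.
; Highlight, visit and unhighlight functions swap materials and set the clickable flag; unhighlight restores either the finish or default material.
; Construction sets the mesh, compares the position to the level's Level_Rules finish tile and caches the default material.
; The finish-material step in construction is disconnected, and GetPlayerCurrentTile is a zero-returning stub.
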(event `/Game/Blueprints/BPI_MyInterface.On_Click`
  (if (`self.is_highlighted`)
    (message `/Game/Blueprints/BPI_MyInterface.Move_Player_To_Tile` (`GameplayStatics.GetPlayerPawn` 0) (`self.K2_GetActorLocation`) (`self.tile_pos`))))

(fn `Get_Player_Current_Tile`
  (returns (tile_pos :type "Vector2D Structure"))
  (return (0.0 0.0)))

(fn `Highlight_Tile`
  (set `self.is_highlighted` true)
  (`PrimitiveComponent.SetMaterial` (`self.tile_mesh`) 0 "/AnimationSharing/AnimSharingGreen.AnimSharingGreen"))

(fn `UnHighlight_Tile`
  (set `self.is_highlighted` false)
  (if (`self.finish_tile`)
    (`PrimitiveComponent.SetMaterial` (`self.tile_mesh`) 0 "/Game/Materials/M_Finish.M_Finish")
    (else
      (`PrimitiveComponent.SetMaterial` (`self.tile_mesh`) 0 (`self.default_material`)))))

(fn `UserConstructionScript`
  (bind _tile_mesh (`self.tile_mesh`))
  (bind (_tile_pos_x _tile_pos_y) (`KismetMathLibrary.BreakVector2D` (`self.tile_pos`)))
  (`StaticMeshComponent.SetStaticMesh` _tile_mesh (`self.New Mesh`))
  (bind _returnvalue (`GameplayStatics.GetCurrentLevelName` true))
  (bind _returnvalue_2 (`|GetDataTableRow` "/Game/Blueprints/Level_Rules.Level_Rules" (`KismetStringLibrary.Conv_StringToName` _returnvalue))
    (:`then`
      _)
    (:`RowNotFound`
      _))
  (bind (_playerstarttile _finishtile) (break `/Game/Blueprints/S_LevelRules` _returnvalue_2))
  (if (and (== (`KismetMathLibrary.BreakVector2D` _finishtile) _tile_pos_x) (== (`.Y` (`KismetMathLibrary.BreakVector2D` _finishtile)) _tile_pos_y))
    _
    (else
      _))
  (set `self.default_material` (`PrimitiveComponent.GetMaterial` _tile_mesh 0)))

(fn `Visit_Tile`
  (set `self.is_highlighted` true)
  (`PrimitiveComponent.SetMaterial` (`self.tile_mesh`) 0 "/AnimationSharing/AnimSharingBlue.AnimSharingBlue"))