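; Player dice for a grid puzzle where the die must reach a finish tile within a move budget from the Level_Rules data table.
; Handles menus, start placement and mouse-trace clicks; clicking the die reads its top face via arrow dot products and has BP_TileGenerator highlight tiles for that number.
; A chosen tile sets a direction, and a timeline tips the cube along highlighted tiles, re-checking after each step, with win/lose feedback.
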(event `Start_Play_Event`
  (bind _returnvalue (`|CreateWidget` "/Game/Blueprints/Widgets/UW_Pausemenu.UW_Pausemenu_C" (`GameplayStatics.GetPlayerController` 0)))
  (bind _output_get (set `self.pause_menu_ui` _returnvalue))
  (`UserWidget.AddToViewport` _output_get 0)
  (`WidgetBlueprintLibrary.SetInputMode_GameAndUIEx` (`GameplayStatics.GetPlayerController` 0) (`self.pause_menu_ui`))
  (bind _returnvalue_2 (`GameplayStatics.GetCurrentLevelName` true))
  (bind _returnvalue_3 (`|GetDataTableRow` "/Game/Blueprints/Level_Rules.Level_Rules" (`KismetStringLibrary.Conv_StringToName` _returnvalue_2))
    (:`then`
      (`/Game/Blueprints/Widgets/UW_Pausemenu.Update_Moves_Text` _output_get (`.NumberofMoves_8_624CCF9741DF49B3EBB49C9A8C054795` (break `/Game/Blueprints/S_LevelRules` _returnvalue_3))))))

(event `self.ReceiveBeginPlay`
  (bind _tile_generator (`self.tile_generator`))
  (bind _lv_rules (`self.lv_rules`))
  (bind (_lv_rules_playerstarttile _lv_rules_finishtile _lv_rules_numberofmoves) (break `/Game/Blueprints/S_LevelRules` (`self.lv_rules`)))
  (`|ExecutionSequence`
    (:`then_0`
      (bind _returnvalue (`|CreateWidget` "/Game/Blueprints/Widgets/UW_MainMenu.UW_MainMenu_C"))
      (`UserWidget.AddToViewport` _returnvalue 0)
      (set `PlayerController.bShowMouseCursor` true (`GameplayStatics.GetPlayerController` 0))
      (`WidgetBlueprintLibrary.SetInputMode_UIOnlyEx` (`GameplayStatics.GetPlayerController` 0) _returnvalue)
      (add `/Game/Blueprints/Widgets/UW_MainMenu.Start_Play` _returnvalue (delegate `Start_Play_Event`)))
    (:`then_1`
      (bind _returnvalue_2 (`GameUserSettings.GetGameUserSettings`))
      (`GameUserSettings.SetScreenResolution` _returnvalue_2 (make `IntPoint` 1080 1920))
      (`GameUserSettings.ApplyResolutionSettings` _returnvalue_2 true)
      (`KismetSystemLibrary.Delay` 0.2)
      (bind _returnvalue_3 (`GameplayStatics.GetCurrentLevelName` true))
      (bind _returnvalue_4 (`|GetDataTableRow` "/Game/Blueprints/Level_Rules.Level_Rules" (`KismetStringLibrary.Conv_StringToName` _returnvalue_3))
        (:`then`
          (bind _output_get (set `self.lv_rules` _returnvalue_4))
          (`SceneComponent.K2_SetRelativeRotation` (`self.Cube_Mesh`) (select `int` (`.Initial_Roll_Number_12_2B38CD294A8306FA21DDA88318357A23` (break `/Game/Blueprints/S_LevelRules` _output_get)) :`0` (struct) :`1` (struct) :`2` (struct) :`3` (struct :`Roll` 180.0) :`4` (struct) :`5` (struct :`Pitch` -90.0 :`Yaw` 180.0) :`6` (struct :`Pitch` -90.0 :`Yaw` -90.0) :!type "Rotator Structure") false false)
          (set `PlayerController.bShowMouseCursor` true (`GameplayStatics.GetPlayerController` 0))
          (`/Engine/EditorBlueprintResources/StandardMacros.IsValid` (`self.tile_generator`)
            (:`Is Valid`
              (if (> (`/Game/Blueprints/BP_TileGenerator.Total_Tiles` _tile_generator) 0) :!label _label
                _
                (else
                  _))
              (bind _array_element (`/Game/Blueprints/BP_TileGenerator.Get_Tile` _tile_generator (`KismetMathLibrary.FTrunc` (`KismetMathLibrary.BreakVector2D` (break `/Game/Blueprints/S_LevelRules` _lv_rules))) (`KismetMathLibrary.FTrunc` (`.Y` (`KismetMathLibrary.BreakVector2D` (break `/Game/Blueprints/S_LevelRules` _lv_rules))))))
              (`/Engine/EditorBlueprintResources/StandardMacros.IsValid` _array_element
                (:`Is Valid`
                  (`self.K2_SetActorLocation` (`self.K2_GetActorLocation` _array_element) false true)
                  (set `self.player_pos` _lv_rules_playerstarttile)
                  (`KismetSystemLibrary.Delay` 0.2)
                  (bind _pause_menu_ui (`self.pause_menu_ui`)
                    (:`then`
                      (`/Game/Blueprints/Widgets/UW_Pausemenu.Update_Moves_Text` _pause_menu_ui _lv_rules_numberofmoves))
                    (:`else`)))))
            (:`Is Not Valid`
              (bind _returnvalue_5 (`GameplayStatics.GetActorOfClass` "/Game/Blueprints/BP_TileGenerator.BP_TileGenerator_C"))
              (bind _output_get_2 (set `self.tile_generator` _returnvalue_5))
              (`/Engine/EditorBlueprintResources/StandardMacros.IsValid` _output_get_2
                (:`Is Valid`
                  (goto _label))
                (:`Is Not Valid`
                  (`self.Create_Tile_Generator`)
                  (`KismetSystemLibrary.PrintString` "Generator Not Found" true true (struct :`R` 1.0 :`G` 0.012294 :`A` 1.0) 10.0))))))
        (:`RowNotFound`
          (`KismetSystemLibrary.PrintString` "Row Not Found" true true (struct :`R` 1.0 :`B` 0.044205 :`A` 1.0) 10.0))))))

(event `Create_Tile_Generator`
  (bind _returnvalue (`|SpawnActorFromClass` "/Game/Blueprints/BP_TileGenerator.BP_TileGenerator_C" (`KismetMathLibrary.MakeTransform` (0.0 0.0 0.0)) "Undefined" "MultiplyWithRoot" null 10 10 null))
  (set `self.tile_generator` _returnvalue))

(event `Key|LeftMouseButton`
  (params (Key :type "Key Structure"))
  (bind _returnvalue (`GameplayStatics.GetPlayerController` 0))
  (bind (_locationx _locationy) (`PlayerController.GetMousePosition` _returnvalue))
  (bind (_worldlocation _worlddirection) (`PlayerController.DeprojectScreenPositionToWorld` _returnvalue _locationx _locationy))
  ; Trace
  (:`Pressed`
    (bind (_outhit _returnvalue_2) (`KismetSystemLibrary.LineTraceSingle` :`Start` _worldlocation :`End` (+ _worldlocation (* _worlddirection 10000000.0)) :`TraceChannel` "TraceTypeQuery3" :`bIgnoreSelf` false :`DrawTime` 500.0))
    (if _returnvalue_2
      (message `/Game/Blueprints/BPI_MyInterface.On_Click` (`.HitActor` (`GameplayStatics.BreakHitResult` _outhit))))))

(event `/Game/Blueprints/BPI_MyInterface.On_Click`
  (`self.Roll_Dice`))

(event `Roll_Dice`
  (bind _rollwed_number (`self.Get_Dice_Number`))
  (if (and (!= _rollwed_number 0) (`self.moved?`) (not (`self.rolling?`)))
    (set `self.moved?` false)
    (bind _output_get (set `self.rolled_number` _rollwed_number))
    (`KismetSystemLibrary.PrintString` (`KismetStringLibrary.Conv_IntToString` _output_get))
    (`/Game/Blueprints/BP_TileGenerator.Highlight_Tiles` (`self.tile_generator`) _output_get)))

(event `/Game/Blueprints/BPI_MyInterface.Move_Player_To_Tile`
  (params (transform :type "Vector Structure") (tile_pos :type "Vector2D Structure"))
  (bind (_lv_rules_playerstarttile _lv_rules_finishtile _lv_rules_numberofmoves) (break `/Game/Blueprints/S_LevelRules` (`self.lv_rules`)))
  (bind (_player_pos_x _player_pos_y) (`KismetMathLibrary.BreakVector2D` (`self.player_pos`)))
  (bind _lv_rules (`self.lv_rules`))
  (bind _pause_menu_ui (`self.pause_menu_ui`))
  (bind _pause_menu_ui_2 (`self.pause_menu_ui`))
  (bind (_lv_rules_playerstarttile_2 _lv_rules_finishtile_2 _lv_rules_numberofmoves_2) (break `/Game/Blueprints/S_LevelRules` (`self.lv_rules`)))
  ; Move Player Dice
  (if (not (`self.rolling?`))
    (bind _dir (`self.Caluclate_Direction` tile_pos))
    (bind _output_get (set `self.move_direction` _dir))
    (`self.Can_Move_Cube` _output_get)
    (if (and (== _player_pos_x (`KismetMathLibrary.BreakVector2D` (`.FinishTile_5_664446CF407DF3BF2870888897255CAD` (break `/Game/Blueprints/S_LevelRules` _lv_rules)))) (== _player_pos_y (`.Y` (`KismetMathLibrary.BreakVector2D` (`.FinishTile_5_664446CF407DF3BF2870888897255CAD` (break `/Game/Blueprints/S_LevelRules` _lv_rules))))))
      (`WidgetBlueprintLibrary.SetInputMode_UIOnlyEx` (`GameplayStatics.GetPlayerController` 0) _pause_menu_ui_2)
      (`/Game/Blueprints/Widgets/UW_Pausemenu.Update_Game_State_Text` _pause_menu_ui_2 true)
      (`GameplayStatics.PlaySound2D` "/Game/Assets/Audio/Level_Complete/universfield-game-level-complete-143022.universfield-game-level-complete-143022" 1.0 1.0 0.0 null null)
      (else
        (setmembers `/Game/Blueprints/S_LevelRules` :`StructRef` (`self.lv_rules`) :`Number of Moves` (- _lv_rules_numberofmoves 1))
        (if (> _lv_rules_numberofmoves_2 0)
          (set `self.moved?` true)
          (`/Game/Blueprints/Widgets/UW_Pausemenu.Update_Moves_Text` _pause_menu_ui _lv_rules_numberofmoves_2)
          (else
            (`/Game/Blueprints/Widgets/UW_Pausemenu.Update_Game_State_Text` _pause_menu_ui false)
            (`GameplayStatics.PlaySound2D` "/Game/Assets/Audio/Level_Fail/u_3bsnvt0dsu-spin-fail-295088.u_3bsnvt0dsu-spin-fail-295088" 1.0 1.0 0.0 null null)))))))

(event `Can_Move_Cube`
  (params (dir :type "/Game/Blueprints/E_MoveDirection Enum" :default "NewEnumerator0"))
  (bind (_player_pos_x _player_pos_y) (`KismetMathLibrary.BreakVector2D` (`self.player_pos`)))
  (bind (_player_pos_x_2 _player_pos_y_2) (`KismetMathLibrary.BreakVector2D` (`self.player_pos`)))
  (bind (_player_pos_x_3 _player_pos_y_3) (`KismetMathLibrary.BreakVector2D` (`self.player_pos`)))
  (bind (_player_pos_x_4 _player_pos_y_4) (`KismetMathLibrary.BreakVector2D` (`self.player_pos`)))
  (switch `/Game/Blueprints/E_MoveDirection` dir
    (:`NewEnumerator0`
      (bind _array_element (`/Game/Blueprints/BP_TileGenerator.Get_Highlighted_Tile` (`self.tile_generator`) (`KismetMathLibrary.FTrunc` _player_pos_x_2) (`KismetMathLibrary.FTrunc` (+ _player_pos_y_2 1.0))))
      (`/Engine/EditorBlueprintResources/StandardMacros.IsValid` _array_element
        (:`Is Valid`
          (if (`/Game/Blueprints/BP_Tile.is_highlighted` _array_element)
            (set `self.player_pos` (`/Game/Blueprints/BP_Tile.tile_pos` _array_element))
            (`self.Update_Pos_Rot` (`self.K2_GetActorLocation` _array_element) (struct :`Roll` 90.0))
            (else
              (`self.End_Move` :!label _label_2))))
        (:`Is Not Valid`
          (goto _label_2))))
    (:`NewEnumerator1`
      (bind _array_element_2 (`/Game/Blueprints/BP_TileGenerator.Get_Highlighted_Tile` (`self.tile_generator`) (`KismetMathLibrary.FTrunc` _player_pos_x_3) (`KismetMathLibrary.FTrunc` (+ _player_pos_y_3 -1.0))))
      (`/Engine/EditorBlueprintResources/StandardMacros.IsValid` _array_element_2
        (:`Is Valid`
          (if (`/Game/Blueprints/BP_Tile.is_highlighted` _array_element_2)
            (set `self.player_pos` (`/Game/Blueprints/BP_Tile.tile_pos` _array_element_2))
            (`self.Update_Pos_Rot` (`self.K2_GetActorLocation` _array_element_2) (struct :`Roll` -90.0))
            (else
              (`self.End_Move` :!label _label_3))))
        (:`Is Not Valid`
          (goto _label_3))))
    (:`NewEnumerator2`
      (bind _array_element_3 (`/Game/Blueprints/BP_TileGenerator.Get_Highlighted_Tile` (`self.tile_generator`) (`KismetMathLibrary.FTrunc` (+ _player_pos_x_4 -1.0)) (`KismetMathLibrary.FTrunc` _player_pos_y_4)))
      (`/Engine/EditorBlueprintResources/StandardMacros.IsValid` _array_element_3
        (:`Is Valid`
          (if (`/Game/Blueprints/BP_Tile.is_highlighted` _array_element_3)
            (set `self.player_pos` (`/Game/Blueprints/BP_Tile.tile_pos` _array_element_3))
            (`self.Update_Pos_Rot` (`self.K2_GetActorLocation` _array_element_3) (struct :`Pitch` 90.0))
            (else
              (`self.End_Move` :!label _label_4))))
        (:`Is Not Valid`
          (goto _label_4))))
    (:`NewEnumerator3`
      (bind _array_element_4 (`/Game/Blueprints/BP_TileGenerator.Get_Highlighted_Tile` (`self.tile_generator`) (`KismetMathLibrary.FTrunc` (+ _player_pos_x 1.0)) (`KismetMathLibrary.FTrunc` _player_pos_y)))
      (`/Engine/EditorBlueprintResources/StandardMacros.IsValid` _array_element_4
        (:`Is Valid`
          (if (`/Game/Blueprints/BP_Tile.is_highlighted` _array_element_4)
            (set `self.player_pos` (`/Game/Blueprints/BP_Tile.tile_pos` _array_element_4))
            (`self.Update_Pos_Rot` (`self.K2_GetActorLocation` _array_element_4) (struct :`Pitch` -90.0))
            (else
              (`self.End_Move` :!label _label_5))))
        (:`Is Not Valid`
          (goto _label_5))))))

(event `End_Move`
  (bind _pause_menu_ui (`self.pause_menu_ui`))
  (bind (_player_pos_x _player_pos_y) (`KismetMathLibrary.BreakVector2D` (`self.player_pos`)))
  (bind _lv_rules (`self.lv_rules`))
  (set `self.moved?` true)
  (`/Game/Blueprints/BP_TileGenerator.Highlight_Tiles` (`self.tile_generator`) 0)
  (if (and (== _player_pos_x (`KismetMathLibrary.BreakVector2D` (`.FinishTile_5_664446CF407DF3BF2870888897255CAD` (break `/Game/Blueprints/S_LevelRules` _lv_rules)))) (== _player_pos_y (`.Y` (`KismetMathLibrary.BreakVector2D` (`.FinishTile_5_664446CF407DF3BF2870888897255CAD` (break `/Game/Blueprints/S_LevelRules` _lv_rules))))))
    (`WidgetBlueprintLibrary.SetInputMode_UIOnlyEx` (`GameplayStatics.GetPlayerController` 0) _pause_menu_ui)
    (`/Game/Blueprints/Widgets/UW_Pausemenu.Update_Game_State_Text` _pause_menu_ui true)
    (`GameplayStatics.PlaySound2D` "/Game/Assets/Audio/Level_Complete/universfield-game-level-complete-143022.universfield-game-level-complete-143022" 1.0 1.0 0.0 null null)))

(event `self.ReceiveTick`
  (params (DeltaSeconds :type "Float (single-precision)"))
  (bind _cube_mesh (`self.Cube_Mesh`))
  (`KismetSystemLibrary.PrintString` (`KismetStringLibrary.Conv_RotatorToString` (`SceneComponent.K2_GetComponentRotation` _cube_mesh)) true true (struct :`G` 0.66 :`B` 1.0 :`A` 1.0) DeltaSeconds)
  (`KismetSystemLibrary.PrintString` (`KismetStringLibrary.Conv_RotatorToString` (`SceneComponent.RelativeRotation` _cube_mesh)) true true (struct :`R` 1.0 :`A` 1.0) DeltaSeconds "bbbb")
  (`KismetSystemLibrary.PrintString` (`KismetStringLibrary.Conv_DoubleToString` (`KismetMathLibrary.Dot_VectorVector` (`SceneComponent.GetForwardVector` (`self.1_Arrow`)) (`self.GetActorUpVector`))) true true (struct :`R` 0.181454 :`G` 1.0 :`B` 0.066692 :`A` 1.0) DeltaSeconds))

(event `Update_Pos_Rot`
  (params (B :type "Vector Structure") (B2 :type "Rotator Structure"))
  (bind _cube_mesh (`self.Cube_Mesh`))
  (bind _returnvalue (/ (.yaw B2) 90.0))
  (bind _returnvalue_2 (/ (.roll B2) 90.0))
  (bind _returnvalue_3 (/ (.pitch B2) 90.0))
  (if (not (`self.rolling?`))
    (set `self.rolling?` true)
    (set `self.current_rotation` (`SceneComponent.K2_GetComponentRotation` (`self.Cube_Mesh`)))
    (set `self.current_location` (`self.K2_GetActorLocation`))
    (bind (_direction _newtrack_0) (`Timeline|Timeline` :!via `PlayFromStart`)
      (:`Update`
        (`self.K2_SetActorLocation` (`KismetMathLibrary.VLerp` (`self.current_location`) B _newtrack_0))
        (`SceneComponent.K2_AddWorldRotation` _cube_mesh (`KismetMathLibrary.MakeRotator` (+ _returnvalue_2 (`self.Get_Speed_Multipler` _returnvalue_2)) (+ _returnvalue_3 (`self.Get_Speed_Multipler` _returnvalue_3)) (+ _returnvalue (`self.Get_Speed_Multipler` _returnvalue))) false false))
      (:`Finished`
        (`/Engine/EditorBlueprintResources/StandardMacros.IncrementInt` (`self.remaining_turns`)
          (:`  `
            (`SceneComponent.K2_SetWorldRotation` (`self.Cube_Mesh`) (`self.current_rotation`) false false)
            (`SceneComponent.K2_AddWorldRotation` _cube_mesh B2 false false)
            (set `self.rolling?` false)
            (`self.Can_Move_Cube` (`self.move_direction`))))))))

(event `Make_Rotation`
  (if (not (`self.is_rot_timmer_running`))
    (set `self.is_rot_timmer_running` true)
    (bind _returnvalue (`KismetSystemLibrary.K2_SetTimerDelegate` (delegate `Cube_Rot`) 0.01 true true))))

(event `Cube_Rot`)

(fn `Caluclate_Direction`
  (params (new_pos :type "Vector2D Structure"))
  (returns (dir :type "/Game/Blueprints/E_MoveDirection Enum"))
  (bind _returnvalue (- new_pos (`self.player_pos`)))
  (bind (_x _y) (`KismetMathLibrary.BreakVector2D` _returnvalue))
  (if (== (`.Y` (`KismetMathLibrary.BreakVector2D` _returnvalue)) 0.0)
    (if (> _x 0.0)
      (return "NewEnumerator3")
      (else
        (return "NewEnumerator2")))
    (elif (> _y 0.0)
      (return "NewEnumerator0")
      (else
        (return "NewEnumerator1")))))

(fn `Get_Dice_Number`
  (returns (rollwed_number :type Integer))
  (if (`KismetMathLibrary.NearlyEqual_FloatFloat` (`KismetMathLibrary.Dot_VectorVector` (`SceneComponent.GetForwardVector` (`self.1_Arrow`)) (`self.GetActorUpVector`)) 1.0)
    (return 1)
    (elif (`KismetMathLibrary.NearlyEqual_FloatFloat` (`KismetMathLibrary.Dot_VectorVector` (`SceneComponent.GetForwardVector` (`self.2_Arrow`)) (`self.GetActorUpVector`)) 1.0)
      (return 2)
      (elif (`KismetMathLibrary.NearlyEqual_FloatFloat` (`KismetMathLibrary.Dot_VectorVector` (`SceneComponent.GetForwardVector` (`self.3_Arrow`)) (`self.GetActorUpVector`)) 1.0)
        (return 3)
        (elif (`KismetMathLibrary.NearlyEqual_FloatFloat` (`KismetMathLibrary.Dot_VectorVector` (`SceneComponent.GetForwardVector` (`self.4_Arrow`)) (`self.GetActorUpVector`)) 1.0)
          (return 4)
          (elif (`KismetMathLibrary.NearlyEqual_FloatFloat` (`KismetMathLibrary.Dot_VectorVector` (`SceneComponent.GetForwardVector` (`self.2_Arrow`)) (`self.GetActorUpVector`)) -1.0)
            (return 5)
            (elif (`KismetMathLibrary.NearlyEqual_FloatFloat` (`KismetMathLibrary.Dot_VectorVector` (`SceneComponent.GetForwardVector` (`self.1_Arrow`)) (`self.GetActorUpVector`)) -1.0)
              (return 6)
              (else
                (return 45)))))))))

(fn `Get_Player_Current_Tile`
  (returns (tile_pos :type "Vector2D Structure"))
  (return (`self.player_pos`)))

(fn `Get_Speed_Multipler`
  (params (C :type "Float (double-precision)"))
  (returns (ReturnValue :type "Float (double-precision)"))
  (return (* (`self.rotation_speed`) (`GameplayStatics.GetWorldDeltaSeconds`) C)))

(fn `Get_Speed_Multipler_0`
  (params (C :type "Float (double-precision)"))
  (returns (ReturnValue :type "Float (double-precision)"))
  (return (* (`self.rotation_speed`) (`GameplayStatics.GetWorldDeltaSeconds`) C)))

(fn `Rot_Equal`
  (params (NewParam :type "Rotator Structure") (NewParam1 :type "Rotator Structure"))
  (returns (ReturnValue :type Boolean))
  (return (and (== (.roll NewParam) (.roll NewParam1)) (== (.pitch NewParam) (.pitch NewParam1)) (== (.yaw NewParam) (.yaw NewParam1)))))

(fn `UserConstructionScript`)